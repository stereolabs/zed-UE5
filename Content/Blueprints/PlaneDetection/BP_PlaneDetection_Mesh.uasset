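; Plane detection actor that turns camera hit tests at mouse clicks into wireframe procedural meshes with collision and places a physics object on them.
; Left click builds the clicked plane's mesh; a normal dot-product check shows the pre-spawned actor on near-horizontal planes, otherwise hides it.
; F builds a separate floor plane mesh.
; The construction script colors both meshes through dynamic material instances.
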(event `self.ReceiveBeginPlay`
  ;[1 1 1] Show mouse
  (set `PlayerController.bShowMouseCursor` true (`ZEDFunctionLibrary.GetPlayerController`))
  ;[1 1 1] Initialize hit tests
  (`SlCameraProxy.EnableHitTest` (`SlFunctionLibrary.GetCameraProxy`) true)
  (`SlCameraProxy.SetHitTestDepthAndNormals` (`SlFunctionLibrary.GetCameraProxy`) true true)
  ;[1 1 1] Prepare spawnable object
  (`self.InitSpawnableActor` (`self.Spawn Transform`)))

(event `self.ReceiveEndPlay`
  (params (EndPlayReason :type "EEndPlayReason Enum" :default "Destroyed"))
  ;[1 1 1] Disable hit test when application quit
  (`SlCameraProxy.EnableHitTest` (`SlFunctionLibrary.GetCameraProxy`) false))

(event `InputAction|MouseLeftClick`
  (params (Key :type "Key Structure"))
  (bind (_locationx _locationy) (`PlayerController.GetMousePosition` (`ZEDFunctionLibrary.GetPlayerController`)))
  (bind (_x _y) (`KismetMathLibrary.BreakVector2D` (`self.MousePosition`)))
  (bind _rootcomponent (`Actor.RootComponent` (`self.SpawnedActor`)))
  (bind (_planelocation _returnvalue) (`ZEDFunctionLibrary.GetFloorPlaneAtScreenPosition` (`ZEDFunctionLibrary.GetPlayerController`) (`KismetMathLibrary.MakeVector2D` _x _y)))
  (bind (_meshdata _returnvalue_2) (`ZEDFunctionLibrary.CreateMeshFromFloorHit` (`ZEDFunctionLibrary.GetPlayerController`) (`KismetMathLibrary.Conv_Vector2DToIntPoint` (`self.MousePosition`))))
  (bind (_vertices _indices) (break `SlMeshData` _meshdata))
  (:`Pressed`
    ;[1 1 1] Retrieve mouse position for plane detection and object spawning
    (set `self.MousePosition` (`KismetMathLibrary.MakeVector2D` _locationx _locationy))
    ;[1 1 1] Test if valid plane
    (if _returnvalue_2
      ;[1 1 1] Display generated plane mesh in the engine from the mesh data
      (`ProceduralMeshComponent.CreateMeshSection_LinearColor` :`self` (`self.PlaneMesh_Wireframe`) :`Vertices` _vertices :`Triangles` _indices :`bCreateCollision` true)
      (if _returnvalue
        (set `self.LocationOnPlane` _planelocation)
        (if (>= (`KismetMathLibrary.Dot_VectorVector` (`ZEDFunctionLibrary.GetNormalAtWorldLocation` (`ZEDFunctionLibrary.GetPlayerController`) _planelocation) (0.0 0.0 1.0)) 0.85)
          ;[1 1 1] Spawn the actor above the plane or hide it
          (`self.ShowHideActor` true)
          (`SceneComponent.K2_SetWorldLocation` _rootcomponent (`self.LocationOnPlane`) false true)
          (`SceneComponent.K2_SetWorldRotation` _rootcomponent (`self.RotationOffset`) false false)
          (else
            (`self.ShowHideActor` false) ; Hide and reset actor if clicked outside a plane
          ))))))

(event `Key|F`
  (params (Key :type "Key Structure"))
  (bind (_vertices _indices) (break `SlMeshData` (`ZEDFunctionLibrary.CreateMeshFromFloorPlane`)))
  ;[1 1 1] Create floor mesh when the F key is pressed
  (:`Pressed`
    (`KismetSystemLibrary.PrintString` "F Pressed, creating floor mesh...")
    (`ProceduralMeshComponent.CreateMeshSection_LinearColor` :`self` (`self.FloorPlaneMesh_Wireframe`) :`Vertices` _vertices :`Triangles` _indices :`bCreateCollision` true)))

(fn `InitSpawnableActor`
  (params (SpawnTransform :type "Transform Structure"))
  (bind _returnvalue (`|SpawnActorFromClass` (`self.Spawnable`) SpawnTransform "Undefined" "OverrideRootScale" null null))
  (bind _output_get (set `self.SpawnedActor` _returnvalue))
  (`SceneComponent.SetVisibility` (`Actor.RootComponent` _output_get) false true)
  (`PrimitiveComponent.SetSimulatePhysics` (`self.GetComponentByClass` (`self.SpawnedActor`) "/Script/Engine.StaticMeshComponent") false))

(fn `ShowHideActor`
  (params (Show :type Boolean))
  (bind _returnvalue (`self.GetComponentByClass` (`self.SpawnedActor`) "/Script/Engine.StaticMeshComponent"))
  (if Show
    (`SceneComponent.SetVisibility` (`Actor.RootComponent` (`self.SpawnedActor`)) true true)
    (`PrimitiveComponent.SetSimulatePhysics` _returnvalue true)
    (`PrimitiveComponent.SetPhysicsLinearVelocity` _returnvalue (0.0 0.0 0.0) false "None")
    (else
      (`SceneComponent.SetVisibility` (`Actor.RootComponent` (`self.SpawnedActor`)) false true)
      (`PrimitiveComponent.SetSimulatePhysics` (`self.GetComponentByClass` (`self.SpawnedActor`) "/Script/Engine.StaticMeshComponent") false)
      (`SceneComponent.K2_SetRelativeLocation` (`Actor.RootComponent` (`self.SpawnedActor`)) (0.0 0.0 0.0) false true))))

(fn `UserConstructionScript`
  (locals (FloorPlaneColor :type "LinearColor Structure" :default (struct :`G` 0.28 :`B` 1.0 :`A` 1.0)) (PlaneColor :type "LinearColor Structure" :default (struct :`R` 0.86 :`G` 0.08 :`B` 0.59 :`A` 1.0)))
  (bind _returnvalue (`KismetMaterialLibrary.CreateDynamicMaterialInstance` "/Game/Materials/PlaneDetection/M_PlaneDetection_Wireframe.M_PlaneDetection_Wireframe"))
  (`MaterialInstanceDynamic.SetVectorParameterValue` _returnvalue "Color" (`local.FloorPlaneColor`))
  (`PrimitiveComponent.SetMaterial` (`self.FloorPlaneMesh_Wireframe`) 0 _returnvalue)
  (bind _returnvalue_2 (`KismetMaterialLibrary.CreateDynamicMaterialInstance` "/Game/Materials/PlaneDetection/M_PlaneDetection_Wireframe.M_PlaneDetection_Wireframe"))
  (`MaterialInstanceDynamic.SetVectorParameterValue` _returnvalue_2 "Color" (`local.PlaneColor`))
  (`PrimitiveComponent.SetMaterial` (`self.PlaneMesh_Wireframe`) 0 _returnvalue_2))