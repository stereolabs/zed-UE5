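; BP_CrosshairOnMouse is a 3D crosshair that follows the visible mouse cursor over surfaces seen by the camera.
; BeginPlay enables the camera proxy's hit test with depth and normals, and EndPlay disables it.
; Tick queries the pixel under the mouse, then places the root along the camera ray, corrected for depth versus distance and pulled forward by CursorOffset for clean occlusion.
; Its rotation follows the surface normal plus RotationOffset.
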(event `self.ReceiveBeginPlay`
  ;[1 1 1] Set cursor visible
  (set `PlayerController.bShowMouseCursor` true (`ZEDFunctionLibrary.GetPlayerController`))
  ;[1 1 1] Enable hit test. Can be done in level blueprint
  (`SlCameraProxy.EnableHitTest` (`SlFunctionLibrary.GetCameraProxy`) true)
  (`SlCameraProxy.SetHitTestDepthAndNormals` (`SlFunctionLibrary.GetCameraProxy`) true true)
  (`self.EnableInput` (`GameplayStatics.GetPlayerController` 0)))

(event `self.ReceiveEndPlay`
  (params (EndPlayReason :type "EEndPlayReason Enum" :default "Destroyed"))
  ;[1 1 1] Always disable hit test before application quit
  (`SlCameraProxy.EnableHitTest` (`SlFunctionLibrary.GetCameraProxy`) false))

(event `self.ReceiveTick`
  (params (DeltaSeconds :type "Float (single-precision)"))
  (bind (_pixelworldlocation _depth _distance _normal) (`ZEDFunctionLibrary.GetPixelLocationAndNormalAtScreenPosition` (`ZEDFunctionLibrary.GetPlayerController`) (`self.MousePosOnScreen`)))
  (bind (_locationx _locationy) (`PlayerController.GetMousePosition` (`ZEDFunctionLibrary.GetPlayerController`)))
  (bind _returnvalue (`SceneComponent.K2_GetComponentLocation` (`Actor.RootComponent` (`ZEDFunctionLibrary.GetCameraActor`))))
  (bind _returnvalue_2 (- _pixelworldlocation _returnvalue))
  (set `self.MousePosOnScreen` (`KismetMathLibrary.MakeVector2D` _locationx _locationy))
  (`SceneComponent.K2_SetWorldLocation` (`self.DefaultSceneRoot`) (+ (* (`KismetMathLibrary.Normal` _returnvalue_2) (- (- (`KismetMathLibrary.VSize` _returnvalue_2) (- _distance _depth)) (`self.CursorOffset`))) _returnvalue) false false)
  (`SceneComponent.K2_SetWorldRotation` (`self.DefaultSceneRoot`) (`KismetMathLibrary.Conv_VectorToRotator` (+ _normal (`self.RotationOffset`))) false false))

(fn `UserConstructionScript`)