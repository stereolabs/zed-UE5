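; BP_HitTestBall is a randomly colored ball that, once thrown, flies until HitTestReal reports a hit.
; Throw stores direction and occlusion offset; while Move is set, Tick offsets the actor at constant speed without sweeping and runs the hit test at its location.
; A hit stops it; with ClampToHitLocation, it snaps to the hit point, backed off by the offset, and enables custom depth stencil rendering.
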(event `Throw`
  (params (Direction :type "Vector Structure") (OcclusionOffset :type "Float (double-precision)"))
  (set `self.Direction` Direction)
  (set `self.OccluOffset` OcclusionOffset))

(event `self.ReceiveTick`
  (params (DeltaSeconds :type "Float (single-precision)"))
  (bind _sphere (`self.Sphere`))
  (bind (_hitresult _returnvalue) (`ZEDFunctionLibrary.HitTestReal` (`ZEDFunctionLibrary.GetPlayerController`) (`self.K2_GetActorLocation`) 15.0 false true))
  (if (`self.bMove`)
    (`self.K2_AddActorWorldOffset` (* (`self.Direction`) (* DeltaSeconds 500.0)))
    (if _returnvalue
      (set `self.bMove` false)
      (if (`self.ClampToHitLocation`)
        (`self.K2_SetActorLocation` self (+ (`.Location` (break `ZEDHitResult` _hitresult)) (* (* (`self.Direction`) (`self.ConstMinus1`)) (`self.OccluOffset`))) false false)
        (`PrimitiveComponent.SetRenderCustomDepth` _sphere true)
        (`PrimitiveComponent.SetCustomDepthStencilValue` _sphere 0)))))

(fn `UserConstructionScript`
  (`MeshComponent.SetVectorParameterValueOnMaterials` (`self.Sphere`) "Color" (`KismetMathLibrary.MakeVector` (`KismetMathLibrary.RandomFloat`) (`KismetMathLibrary.RandomFloat`) (`KismetMathLibrary.RandomFloat`))))