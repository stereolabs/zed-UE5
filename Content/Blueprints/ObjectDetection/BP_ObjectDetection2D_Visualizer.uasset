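; Visualizer actor that draws 2D bounding boxes of objects detected by the camera on screen.
; On BeginPlay it adds a BP_BBox2D widget to the viewport and binds camera proxy events, passing the camera resolution and each set of retrieved objects to the widget.
; Detection optionally starts when tracking is enabled, and custom events allow enabling or disabling it manually from the editor.
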(event `Disable OD`
  ;[1 1 1] Create Enable/Disable OD button in Editor
  (`ZEDCamera.DisableObjectDetection` (`ZEDFunctionLibrary.GetCameraActor`)))

(event `Enable OD`
  ;[1 1 1] Create Enable/Disable OD button in Editor
  (`ZEDCamera.EnableObjectDetection` (`ZEDFunctionLibrary.GetCameraActor`)))

(event `self.ReceiveBeginPlay`
  (`|ExecutionSequence`
    (:`then_0`
      ;[1 1 1] Add Widget used to draw bboxes to Viewport
      (bind _returnvalue (`|CreateWidget` "/Game/Blueprints/ObjectDetection/BP_BBox2D.BP_BBox2D_C"))
      (bind _output_get (set `self.Bboxes2D` _returnvalue))
      (`UserWidget.AddToViewport` _output_get 0)
      ;[1 1 1] Retrieve Camera resolution at open
      (add `SlCameraProxy.OnCameraOpened` (`SlFunctionLibrary.GetCameraProxy`) (delegate `OnCameraOpened_Event_0`)))
    (:`then_1`
      ;[1 1 1] Bind event to retrieve object function
      (add `SlCameraProxy.OnObjectDetectionRetrieved` (`SlFunctionLibrary.GetCameraProxy`) (delegate `OnObjectDetectionRetrieved_Event_1`)))
    (:`then_2`
      ;[1 1 1] Enable OD automaticcly when the camera is ready (when tracking is enabled)
      (add `SlCameraProxy.OnTrackingEnabled` (`SlFunctionLibrary.GetCameraProxy`) (delegate `OnTrackingEnabled_Event_0`)))))

(event `OnCameraOpened_Event_0`
  ;[1 1 1] Retrieve Camera resolution at open
  (set `/Game/Blueprints/ObjectDetection/BP_BBox2D.CameraResolution` (`.Resolution` (break `SlCameraInformation` (`SlCameraProxy.CameraInformation` (`SlFunctionLibrary.GetCameraProxy`)))) (`self.Bboxes2D`)))

(event `OnObjectDetectionRetrieved_Event_1`
  (params (objects :type "SlObjects Structure (by ref)"))
  ;[1 1 1] Bind event to retrieve object function
  (set `/Game/Blueprints/ObjectDetection/BP_BBox2D.Objects` objects (`self.Bboxes2D`)))

(event `OnTrackingEnabled_Event_0`
  (params (bSuccess :type Boolean) (ErrorCode :type "ESlErrorCode Enum" :default "EC_Success") (Location :type "Vector Structure (by ref)") (Rotation :type "Rotator Structure (by ref)"))
  ;[1 1 1] Enable OD automaticcly when the camera is ready (when tracking is enabled)
  (if (`self.Start Object Detection Automatically`)
    (`ZEDCamera.EnableObjectDetection` (`ZEDFunctionLibrary.GetCameraActor`))))

(fn `UserConstructionScript`)