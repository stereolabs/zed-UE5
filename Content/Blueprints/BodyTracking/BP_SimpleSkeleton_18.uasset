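; Body-tracking skeleton actor that displays 18 keypoints as small spheres.
; On BeginPlay it spawns and attaches the BP_CustomSphere nodes, each given a random color as a placeholder for per-joint coloring.
; MoveNodesToKeypoints places them at supplied world locations, remapping 34-keypoint input through KPs18in34 and otherwise using indices directly.
; ShowNodes toggles the spheres' visibility, along with their collision between physics-only and none.
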(event `self.ReceiveBeginPlay`
  ;[1 1 1] Fill array of node actors (spheres)
  (for _index (range 18)
    (bind _returnvalue (`|SpawnActorFromClass` "/Game/Blueprints/BodyTracking/BP_CustomSphere.BP_CustomSphere_C" (`KismetMathLibrary.MakeTransform` (`SceneComponent.K2_GetComponentLocation` (`self.DefaultSceneRoot`)) (struct) (0.1 0.1 0.1)) "AlwaysSpawn" "OverrideRootScale" null null))
    (`MeshComponent.SetVectorParameterValueOnMaterials` (`StaticMeshActor.StaticMeshComponent` _returnvalue) "MaterialColor" (`self.GiveColorDependingOnIndex` _index))
    (`self.K2_AttachToActor` _returnvalue self "None" "KeepRelative" "KeepRelative" "KeepRelative" true)
    (`KismetArrayLibrary.Array_Add` (`self.Nodes`) _returnvalue)))

(fn `GiveColorDependingOnIndex`
  (params (Index :type Integer))
  (returns (Color :type "Vector Structure"))
  ;[1 1 1] Todo : distribuer couleur selon node
  (return (`KismetMathLibrary.RandomUnitVector`)))

(fn `MoveNodesToKeypoints`
  (params (KeypointsLocations :type "Array of Vector Structure"))
  (locals (KPs18in34 :type "Array of Integer") (Counter34 :type Integer))
  (set `self.KeypointsLocs` KeypointsLocations)
  (if (== (`KismetArrayLibrary.Array_Length` KeypointsLocations) 34)
    (for (_ _array_index) (`self.Nodes`)
      (`self.MoveNodeTo` _array_index (`|GetArrayItem` (`self.KeypointsLocs`) (`|GetArrayItem` (`local.KPs18in34`) _array_index))))
    (else
      ;[1 1 1] 18 keypoints
      (for (_ _array_index_2) (`self.Nodes`)
        (`self.MoveNodeTo` _array_index_2 (`|GetArrayItem` (`self.KeypointsLocs`) _array_index_2))))))

(fn `MoveNodeTo`
  (params (IndexNode :type Integer) (NewLocation :type "Vector Structure"))
  (`SceneComponent.K2_SetWorldLocation` (`Actor.RootComponent` (`|GetArrayItem` (`self.Nodes`) IndexNode)) NewLocation false false))

(fn `ShowNodes`
  (params (ShouldShow :type Boolean))
  (if ShouldShow
    (for _array_element (`self.Nodes`)
      (bind _returnvalue (`self.GetComponentByClass` _array_element "/Script/Engine.StaticMeshComponent"))
      (`PrimitiveComponent.SetCollisionEnabled` _returnvalue "PhysicsOnly")
      (`SceneComponent.SetVisibility` _returnvalue ShouldShow false)
      (set `self.IsNodesVisible` ShouldShow))
    (else
      (for _array_element_2 (`self.Nodes`)
        (bind _returnvalue_2 (`self.GetComponentByClass` _array_element_2 "/Script/Engine.StaticMeshComponent"))
        (`PrimitiveComponent.SetCollisionEnabled` _returnvalue_2 "NoCollision")
        (`SceneComponent.SetVisibility` _returnvalue_2 ShouldShow false)
        (set `self.IsNodesVisible` ShouldShow)))))

(fn `UserConstructionScript`)