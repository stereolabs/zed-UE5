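; Body-tracking skeleton manager that adds click-to-spawn props at a tracked avatar's joint, extending its parent manager.
; Left click takes the first entry in the Avatars map and proceeds only if its skeleton has more than 18 keypoints (the 34-point format).
; SpawnThingAtLocation spawns a random Spawnables class at keypoint 7 plus an offset, then gives physics cubes a random material color.
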(event `self.ReceiveBeginPlay`
  (`parent.ReceiveBeginPlay`)
  (`self.EnableInput` (`GameplayStatics.GetPlayerController` 0)))

(event `InputAction|MouseLeftClick`
  (params (Key :type "Key Structure"))
  (:`Pressed`
    (if (> (`BlueprintMapLibrary.Map_Length` (`self.Avatars`)) 0)
      (bind _keys (`BlueprintMapLibrary.Map_Keys` (`self.Avatars`)))
      (bind _asbp_avatar (cast `/Game/Blueprints/BodyTracking/BP_Avatar` (`BlueprintMapLibrary.Map_Find` (`self.Avatars`) (`|GetArrayItem` _keys))))
      (bind (_id _uniqueobjectid _rawlabel _label _sublabel _trackingstate _actionstate _position _velocity _positioncovariance _boundingbox2d _mask _confidence _boundingbox _dimensions _keypoint2d _keypoint) (break `SlObjectData` (`/Game/Blueprints/BodyTracking/BP_Avatar.ObjectData` _asbp_avatar)))
      ;[1 1 1] True - 34 / False - 18
      (if (> (`KismetArrayLibrary.Array_Length` _keypoint) 18)
        (`self.SpawnThingAtLocation` (`|GetArrayItem` _keypoint 7))))))

(fn `SpawnThingAtLocation`
  (params (SpawnLocation :type "Vector Structure"))
  (bind _spawnables (`self.Spawnables`))
  (bind _returnvalue (`|SpawnActorFromClass` (`|GetArrayItem` _spawnables (`KismetMathLibrary.RandomInteger` (`KismetArrayLibrary.Array_Length` _spawnables))) (`KismetMathLibrary.Conv_VectorToTransform` (+ SpawnLocation (`self.CubeSpawnOffset`))) "AlwaysSpawn" "OverrideRootScale" null null))
  (bind _asbp_custom_cube_with_physics (cast `/Game/Blueprints/BodyTracking/BP_CustomCubeWithPhysics` _returnvalue))
  (`MeshComponent.SetVectorParameterValueOnMaterials` (`StaticMeshActor.StaticMeshComponent` _asbp_custom_cube_with_physics) "MaterialColor" (`KismetMathLibrary.RandomUnitVector`)))

(fn `UserConstructionScript`
  (`parent.UserConstructionScript`))