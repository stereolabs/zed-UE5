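; BP_Capsule is a body-tracking actor that stretches itself between two points, apparently to visualize a segment such as a limb.
; Its MoveTo function aims the actor's Z axis from one location toward the other and places it at their midpoint.
; It then scales Z by the distance divided by 100, multiplied by a CustomScaleFactor; the event graph and construction script are empty.
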(fn `MoveTo`
  (params (Location1 :type "Vector Structure") (Location2 :type "Vector Structure"))
  (bind _returnvalue (- Location1 Location2))
  (bind _output_get (set `self.Rotation` (.rotation (`KismetAnimationLibrary.K2_LookAt` (`KismetMathLibrary.Conv_VectorToTransform` Location1) Location2 (0.0 0.0 1.0) false (0.0 0.0 1.0)))))
  (`self.K2_SetActorRotation` _output_get)
  (set `self.Length` (`KismetMathLibrary.VSize` _returnvalue))
  (bind _output_get_2 (set `self.Center` (+ (/ _returnvalue (2.0 2.0 2.0)) Location2)))
  (`self.K2_SetActorLocation` _output_get_2)
  (`self.SetActorRelativeScale3D` (* (`self.CustomScaleFactor`) (`KismetMathLibrary.MakeVector` 1.0 1.0 (/ (`self.Length`) 100.0)))))

(fn `UserConstructionScript`)