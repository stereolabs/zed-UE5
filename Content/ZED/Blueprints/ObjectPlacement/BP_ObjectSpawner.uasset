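; BP_ObjectSpawner spawns random objects into the ZED camera's view of the real scene wherever the left mouse button is clicked.
; BeginPlay shows the cursor and enables camera hit tests with depth and normals, which EndPlay disables.
; Clicks resolve to either a detected floor plane or the pixel's world location and normal, depending on OnlySpawnOnFloor.
; SpawnThingAtLocation offsets a random Spawnables class along that normal and randomizes its MaterialColor.
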(event `self.ReceiveBeginPlay`
  ;[1 1 1] Show mouse
  (set `PlayerController.bShowMouseCursor` true (`ZEDFunctionLibrary.GetPlayerController`))
  ;[1 1 1] Initialize hit tests
  (`SlCameraProxy.EnableHitTest` (`SlFunctionLibrary.GetCameraProxy`) true)
  (`SlCameraProxy.SetHitTestDepthAndNormals` (`SlFunctionLibrary.GetCameraProxy`) true true)
  (`self.EnableInput` (`ZEDFunctionLibrary.GetPlayerController`)))

(event `self.ReceiveEndPlay`
  (params (EndPlayReason :type "EEndPlayReason Enum" :default "Destroyed"))
  ;[1 1 1] Disable hit test when application quit
  (`SlCameraProxy.EnableHitTest` (`SlFunctionLibrary.GetCameraProxy`) false))

(event `InputAction|MouseLeftClick`
  (params (Key :type "Key Structure"))
  (bind (_locationx _locationy) (`PlayerController.GetMousePosition` (`ZEDFunctionLibrary.GetPlayerController`)))
  (bind (_x _y) (`KismetMathLibrary.BreakVector2D` (`self.MousePosition`)))
  (bind (_planelocation _returnvalue) (`ZEDFunctionLibrary.GetFloorPlaneAtScreenPosition` (`ZEDFunctionLibrary.GetPlayerController`) (`KismetMathLibrary.MakeVector2D` _x _y)))
  (:`Pressed`
    ;[1 1 1] Retrieve mouse position for plane detection and object spawning
    (bind _output_get (set `self.MousePosition` (`KismetMathLibrary.MakeVector2D` _locationx _locationy)))
    (if (`self.OnlySpawnOnFloor`)
      (if _returnvalue
        (`self.SpawnThingAtLocation` _planelocation (`KismetMathLibrary.Vector_Up`)))
      (else
        (bind (_pixelworldlocation _depth _distance _normal) (`ZEDFunctionLibrary.GetPixelLocationAndNormalAtScreenPosition` (`ZEDFunctionLibrary.GetPlayerController`) _output_get))
        (`self.SpawnThingAtLocation` _pixelworldlocation _normal)))))

(fn `SpawnThingAtLocation`
  (params (SpawnLocation :type "Vector Structure") (UnitNormal :type "Vector Structure"))
  (bind _spawnables (`self.Spawnables`))
  (bind _returnvalue (`|SpawnActorFromClass` (`|GetArrayItem` _spawnables (`KismetMathLibrary.RandomInteger` (`KismetArrayLibrary.Array_Length` _spawnables))) (`KismetMathLibrary.Conv_VectorToTransform` (+ SpawnLocation (* UnitNormal (`self.SpawnOffset`)))) "AlwaysSpawn" "OverrideRootScale" null null))
  (`MeshComponent.SetVectorParameterValueOnMaterials` (`self.GetComponentByClass` _returnvalue "/Script/Engine.StaticMeshComponent") "MaterialColor" (`KismetMathLibrary.RandomUnitVector`)))

(fn `UserConstructionScript`)