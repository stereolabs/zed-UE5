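; Manager actor that visualizes ZED camera body tracking as animated avatars, one per detected person.
; On BeginPlay it adds a canvas widget for the ZED image and binds to camera events, optionally auto-starting object detection.
; Each detection update spawns avatars by selected body mode, feeds tracked ones animation, smoothing and IK settings, and destroys vanished ones via an ID-keyed map.
; Also exposes detection on/off and avatar visibility events.
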(event `DisableOD`
  ;[1 1 1] Create Enable/Disable OD button in Editor
  (`ZEDCamera.DisableObjectDetection` (`ZEDFunctionLibrary.GetCameraActor`)))

(event `EnableOD`
  ;[1 1 1] Create Enable/Disable OD button in Editor
  (`ZEDCamera.EnableObjectDetection` (`ZEDFunctionLibrary.GetCameraActor`)))

(event `DoOnTrackingEnabled`
  (params (bSuccess :type Boolean) (ErrorCode :type "ESlErrorCode Enum" :default "EC_Success") (Location :type "Vector Structure (by ref)") (Rotation :type "Rotator Structure (by ref)"))
  ;[1 1 1] Enable OD automatically when the camera is ready (when tracking is enabled)
  (if (`self.StartObjectDetectionAutomatically`)
    (`ZEDCamera.EnableObjectDetection` (`ZEDFunctionLibrary.GetCameraActor`))))

(event `self.ReceiveBeginPlay`
  (`|ExecutionSequence`
    (:`then_0`
      ;[1 1 1] Enable OD automatically when the camera is ready (when tracking is enabled)
      (add `SlCameraProxy.OnTrackingEnabled` (`SlFunctionLibrary.GetCameraProxy`) (delegate `DoOnTrackingEnabled`)))
    (:`then_1`
      ;[1 1 1] Create canvas to display ZED Image on the screen
      (bind _returnvalue (`|CreateWidget` "/Game/ZED/Blueprints/BodyTracking/BP_VirtualCanvas.BP_VirtualCanvas_C"))
      (`UserWidget.AddToViewport` _returnvalue 0))
    (:`then_2`
      ;[1 1 1] Bind event to retrieve object function
      (add `SlCameraProxy.OnObjectDetectionRetrieved` (`SlFunctionLibrary.GetCameraProxy`) (delegate `DoOnObjectDetectionRetrieved`)))))

(event `DoOnObjectDetectionRetrieved`
  (params (objects :type "SlObjects Structure (by ref)"))
  (bind (_timestamp _objectslist _bisnew) (break `SlObjects` objects))
  (bind (_value _returnvalue) (`BlueprintMapLibrary.Map_Find` (`self.BodyModeActorClasses`) (`self.SelectedBodyMode`)))
  ;[1 1 1] Bind event to retrieve object function
  (if _bisnew
    ;[1 1 1] Fill up the RemaningAvatars array.
    ; Used to know which person is no longer detected in the scene and destroy its avatar
    (bind _keys (`BlueprintMapLibrary.Map_Keys` (`self.Avatars`)))
    (set `self.Remaining Avatars` _keys)
    ;[1 1 1] Get SlObject and check tracking state
    (for _array_element _objectslist
      (set `self.Current Object` _array_element)
      (bind (_id _uniqueobjectid _rawlabel _label _sublabel _trackingstate) (break `SlObjectData` _array_element))
      (set `self.Id` _id)
      (if (`|EnumEquality` _trackingstate "OTS_Ok")
        ;[1 1 1] Check if new detection or already tracked
        (if (`BlueprintMapLibrary.Map_Contains` (`self.Avatars`) _id)
          ;[1 1 1] If the Avatar is already in the scene, update its animation parameters
          (`KismetArrayLibrary.Array_RemoveItem` (`self.Remaining Avatars`) (`self.Id`))
          (bind _asbp_zed_body_tracking_parent (cast `/Game/ZED/Blueprints/UpperBody/BP_ZED_BodyTrackingParent` (`BlueprintMapLibrary.Map_Find` (`self.Avatars`) (`self.Id`))))
          (`/Game/ZED/Blueprints/UpperBody/BP_ZED_BodyTrackingParent.SetAnimParams` _asbp_zed_body_tracking_parent (`self.Current Object`) (`self.Mirror on ZAxis`) (`self.Stick Avatar on Floor`) (`self.Bone Scaling - Experimental`) (`self.Height Offset`) (`self.JointRotationSmoothing`) (`self.RootTranslationSmoothing`) (`self.EnableFootIK`))
          (else
            ;[1 1 1] New Detection : Spawn a new Avatar and update its Skeletal Mesh with Body Tracking Data
            (if _returnvalue
              (bind _returnvalue_2 (`|SpawnActorFromClass` _value (`self.Spawn Transform`) "Undefined" "OverrideRootScale" null null))
              (`BlueprintMapLibrary.Map_Add` (`self.Avatars`) (`self.Id`) _returnvalue_2)
              (bind _asbp_zed_body_tracking_parent_2 (cast `/Game/ZED/Blueprints/UpperBody/BP_ZED_BodyTrackingParent` _returnvalue_2)
                (:`then`
                  (`/Game/ZED/Blueprints/UpperBody/BP_ZED_BodyTrackingParent.SetAvatarVisibility` _asbp_zed_body_tracking_parent_2 (`self.AvatarsVisible`))
                  (`/Game/ZED/Blueprints/UpperBody/BP_ZED_BodyTrackingParent.SetSelfCollisionActive` _asbp_zed_body_tracking_parent_2 (`self.EnableSelfCollision`))
                  (`/Game/ZED/Blueprints/UpperBody/BP_ZED_BodyTrackingParent.SetAnimParams` _asbp_zed_body_tracking_parent_2 (`self.Current Object`) (`self.Mirror on ZAxis`) (`self.Stick Avatar on Floor`) (`self.Bone Scaling - Experimental`) (`self.Height Offset`) (`self.JointRotationSmoothing`) (`self.RootTranslationSmoothing`) (`self.EnableFootIK`)))
                (:`CastFailed`
                  (`KismetSystemLibrary.PrintString` "Cast to BP_ZED_BTParent failed... The avatar will not be updated!")))
              (else
                (`KismetSystemLibrary.PrintString` "No matching actor class to provided ActorClasses key.")))))))
    ;[1 0.06029 0 0.5] Destroy Avatars which are not longer detected in the scene
    (for _array_element_2 (`self.Remaining Avatars`)
      (bind (_value_2 _returnvalue_3) (`BlueprintMapLibrary.Map_Find` (`self.Avatars`) _array_element_2))
      (if (== _returnvalue_3 true)
        (`self.K2_DestroyActor` _value_2)
        (`BlueprintMapLibrary.Map_Remove` (`self.Avatars`) _array_element_2)))))

(event `ToggleAvatarVisibility`
  (params (Visibility :type Boolean))
  ;[0 0.2871 1] Toggle avatar visibility
  (set `self.AvatarsVisible` Visibility)
  (`KismetSystemLibrary.PrintString` (`KismetStringLibrary.Concat_StrStr` "Avatar ToggleVisibility [" (`KismetStringLibrary.Conv_BoolToString` Visibility) "]"))
  (bind _values (`BlueprintMapLibrary.Map_Values` (`self.Avatars`)))
  (for _array_element _values
    (bind _asbp_zed_body_tracking_parent (cast `/Game/ZED/Blueprints/UpperBody/BP_ZED_BodyTrackingParent` _array_element)
      (:`then`
        (`/Game/ZED/Blueprints/UpperBody/BP_ZED_BodyTrackingParent.SetAvatarVisibility` _asbp_zed_body_tracking_parent Visibility))
      (:`CastFailed`
        (`KismetSystemLibrary.PrintString` "Cast to BP_ZED_BTParent failed!")
        (`SceneComponent.SetVisibility` (`self.GetComponentByClass` _array_element "/Script/Engine.SkeletalMeshComponent") Visibility true)))))

(fn `UpdateSmoothingParams`
  (params (ABP_ZED_Manny :type "/Game/ZED/Blueprints/BodyTracking/ABP_ZED_Manny Object Reference"))
  (set `/Game/ZED/Blueprints/BodyTracking/ABP_ZED_Manny.Rotation Slerp Intensity` (`self.JointRotationSmoothing`) ABP_ZED_Manny)
  (set `/Game/ZED/Blueprints/BodyTracking/ABP_ZED_Manny.Root Location Slerp Intensity` (`self.RootTranslationSmoothing`) ABP_ZED_Manny))

(fn `UserConstructionScript`)