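; Upper-body ZED avatar Blueprint that drives a skeletal mesh through the ABP_ZED_Manny_UpperBody animation Blueprint.
; SetAnimParams forwards object data, mirroring, height offset, bone scaling, smoothing and foot IK settings to that animation instance.
; Enabling self-collision waits briefly, then adds a Physical Animation component and simulates bodies below Hips with full physics blend.
; A visibility override also shows or hides the mesh.
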(event `self.ReceiveBeginPlay`
  (`parent.ReceiveBeginPlay`)
  (set `self.AnimationBlueprint` (cast `/Game/ZED/Blueprints/UpperBody/ABP_ZED_Manny_UpperBody` (`SkeletalMeshComponent.GetAnimInstance` (`self.SkeletalMesh`)) :!pure true)))

(event `EnableSelfCollision`
  (bind _hips (`self.Hips`))
  (`KismetSystemLibrary.Delay` 1.0)
  (bind _returnvalue (`AddComponent|NODE_AddPhysicalAnimationComponent-0`))
  (bind _output_get (set `self.Physical Animation Component` _returnvalue))
  (`PhysicalAnimationComponent.SetSkeletalMeshComponent` _output_get (`self.SkeletalMesh`))
  (`SkeletalMeshComponent.SetAllBodiesBelowSimulatePhysics` (`self.SkeletalMesh`) _hips true false)
  (`SkeletalMeshComponent.SetAllBodiesBelowPhysicsBlendWeight` (`self.SkeletalMesh`) _hips 1.0 false false)
  (`PhysicalAnimationComponent.ApplyPhysicalAnimationSettingsBelow` (`self.Physical Animation Component`) (`self.Hips`) (make `PhysicalAnimationData` false 1000.0 100.0 100.0 100.0) false))

(fn `SetAnimParams`
  (params (ObjectData :type "SlObjectData Structure") (MirrorOnZAxis :type Boolean) (AutomaticHeightOffset :type Boolean) (BoneScaling :type Boolean) (HeightOffset :type "Float (double-precision)") (JointsRotationSlerpFactor :type "Float (double-precision)") (RootLocationLerpFactor :type "Vector Structure") (EnableFootIK :type Boolean))
  (`/Game/ZED/Blueprints/UpperBody/ABP_ZED_Manny_UpperBody.Set Anim Variables` (`self.AnimationBlueprint`) ObjectData MirrorOnZAxis AutomaticHeightOffset BoneScaling HeightOffset JointsRotationSlerpFactor RootLocationLerpFactor EnableFootIK)
  (set `/Game/ZED/Blueprints/UpperBody/ABP_ZED_Manny_UpperBody.Skeletal Mesh` (`self.SkeletalMesh`) (`self.AnimationBlueprint`)))

(fn `SetAvatarVisibility`
  (params (NewVisibility :type Boolean))
  (`parent.SetAvatarVisibility` NewVisibility)
  (`SceneComponent.SetVisibility` (`self.SkeletalMesh`) NewVisibility false))

(fn `SetSelfCollisionActive`
  (params (NewSelfCollisionStatus :type Boolean))
  (`parent.SetSelfCollisionActive` NewSelfCollisionStatus)
  (if NewSelfCollisionStatus
    (`self.EnableSelfCollision`)))

(fn `UserConstructionScript`
  (`parent.UserConstructionScript`))