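; NPC character Blueprint that wanders at random across the navigation mesh at a slow walk speed, which it sets on BeginPlay.
; MoveNPC picks a random reachable point near the actor and sends it there with AIMoveTo.
; Success and failure both re-call MoveNPC after a short delay, forming an endless loop, though nothing in this graph makes the first call.
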(event `self.ReceiveBeginPlay`
  (set `CharacterMovementComponent.MaxWalkSpeed` 40.0 (`self.CharacterMovement`)))

(event `MoveNPC`
  (bind _output_get (set `self.Random Location` (`NavigationSystemV1.K2_GetRandomReachablePointInRadius` (`self.K2_GetActorLocation`) 500.0 null "/Script/AIModule.NavFilter_AIControllerDefault")))
  (`|AIMoveTo` self _output_get null
    (:`OnSuccess`
      (`KismetSystemLibrary.Delay` 0.2)
      (`self.MoveNPC`))
    (:`OnFail`
      (`KismetSystemLibrary.Delay` 0.1)
      (`self.MoveNPC`))))

(fn `UserConstructionScript`)