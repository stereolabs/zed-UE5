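; ZED spatial mapping mesh Blueprint that displays the scanned environment through two procedural meshes, preview and render.
; Initialize binds once to SpatialMappingManager events for mesh updates, filtering, loading, texturing, reset and show/hide.
; Untextured data rebuilds PreviewMesh; textured data rebuilds RenderMesh with a dynamic material, both with optional collision, while load, texturing and reset switch which is shown.
; Both texturing events use MIDRender, leaving the created MIDCubemap unused.
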(event `Initialize`
  (params (SpatialMappingManager :type "/Game/ZED/Blueprints/SpatialMapping/BP_SpatialMapping_Manager Object Reference"))
  (`/Engine/EditorBlueprintResources/StandardMacros.DoOnce` false
    (:`Completed`
      (`self.ResetMeshes`)
      (add `SpatialMappingManager.OnMeshUpdated` SpatialMappingManager (delegate `OnMeshUpdated_Event_0`))
      (add `SpatialMappingManager.OnMeshFiltered` SpatialMappingManager (delegate `OnMeshFiltered_Event_0`))
      (add `SpatialMappingManager.OnMeshLoaded` SpatialMappingManager (delegate `OnMeshLoaded_Event_0`))
      (add `SpatialMappingManager.OnMeshTexturedForCubemap` SpatialMappingManager (delegate `OnMeshTexturedForCubemap_Event_0`))
      (add `SpatialMappingManager.OnMeshTexturedForRendering` SpatialMappingManager (delegate `OnMeshTexturedForRendering_Event_0`))
      (add `SpatialMappingManager.OnSpatialMappingReset` SpatialMappingManager (delegate `OnSptialMappingReset_Event_0`))
      (add `SpatialMappingManager.OnShowMesh` SpatialMappingManager (delegate `OnShowMeshEvent_0`))
      (add `SpatialMappingManager.OnHideMesh` SpatialMappingManager (delegate `OnHideMeshEvent_0`)))))

(event `OnMeshUpdated_Event_0`
  (params (MeshData :type "SlMeshData Structure (by ref)"))
  (`self.UpdatePreviewMesh` MeshData))

(event `OnMeshFiltered_Event_0`
  (params (MeshData :type "SlMeshData Structure (by ref)"))
  (`self.UpdatePreviewMesh` MeshData))

(event `OnMeshLoaded_Event_0`
  (params (MeshData :type "SlMeshData Structure (by ref)"))
  (`self.UpdatePreviewMesh` MeshData)
  (`SceneComponent.SetHiddenInGame` (`self.PreviewMesh`) false false)
  (`SceneComponent.SetHiddenInGame` (`self.RenderMesh`) true false))

(event `OnMeshTexturedForCubemap_Event_0`
  (params (MeshData :type "SlMeshData Structure (by ref)"))
  (`self.UpdateRenderMesh` (`self.MID_Render`) MeshData)
  (`SceneComponent.SetHiddenInGame` (`self.PreviewMesh`) true false :!label _label)
  (`SceneComponent.SetHiddenInGame` (`self.RenderMesh`) false false))

(event `OnMeshTexturedForRendering_Event_0`
  (params (MeshData :type "SlMeshData Structure (by ref)"))
  (`self.UpdateRenderMesh` (`self.MID_Render`) MeshData)
  (goto _label))

(event `OnSptialMappingReset_Event_0`
  (`self.ResetMeshes`)
  (`SceneComponent.SetHiddenInGame` (`self.PreviewMesh`) false false)
  (`SceneComponent.SetHiddenInGame` (`self.RenderMesh`) true false))

(event `OnShowMeshEvent_0`
  (`ProceduralMeshComponent.SetMeshSectionVisible` (`self.PreviewMesh`) 0 true)
  (`ProceduralMeshComponent.SetMeshSectionVisible` (`self.RenderMesh`) 0 true))

(event `OnHideMeshEvent_0`
  (`ProceduralMeshComponent.SetMeshSectionVisible` (`self.PreviewMesh`) 0 false)
  (`ProceduralMeshComponent.SetMeshSectionVisible` (`self.RenderMesh`) 0 false))

(event `ResetMeshes`
  (`ProceduralMeshComponent.ClearAllMeshSections` (`self.RenderMesh`))
  (`ProceduralMeshComponent.ClearAllMeshSections` (`self.PreviewMesh`)))

(fn `UserConstructionScript`
  (`|ExecutionSequence`
    (:`then_0`
      (bind _returnvalue (`KismetMaterialLibrary.CreateDynamicMaterialInstance` "/Game/ZED/Materials/SpatialMapping/M_SpatialMapping_RenderMesh.M_SpatialMapping_RenderMesh"))
      (set `self.MID_Render` _returnvalue)
      (bind _returnvalue_2 (`KismetMaterialLibrary.CreateDynamicMaterialInstance` "/Game/ZED/Materials/SpatialMapping/M_SpatialMapping_RenderMeshCubemap.M_SpatialMapping_RenderMeshCubemap"))
      (set `self.MID_Cubemap` _returnvalue_2))
    (:`then_1`
      (`PrimitiveComponent.SetMaterial` (`self.PreviewMesh`) 0 "/Game/ZED/Materials/SpatialMapping/M_SpatialMapping_PreviewMesh.M_SpatialMapping_PreviewMesh"))))