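; 3D bounding box Blueprint for ZED object detection, with a box mesh, a bordered label background and a text render.
; On BeginPlay it picks a random color from a fixed palette.
; It applies that color through dynamic material instances on the box and border, and sets the text color to match.
; This graph only handles coloring and contains no logic for placement, sizing or label content.
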(event `self.ReceiveBeginPlay`
  (set `self.Color` (`KismetArrayLibrary.Array_Random` (`|MakeArray` (`KismetMathLibrary.MakeColor` 0.231 0.909 0.69) (`KismetMathLibrary.MakeColor` 0.098039 0.686 0.816) (`KismetMathLibrary.MakeColor` 0.412 0.4 0.804) (`KismetMathLibrary.MakeColor` 1.0 0.725) (`KismetMathLibrary.MakeColor` 0.098824 0.388 0.419))))
  ;[1 1 1] Set color of the bbox
  (bind _returnvalue (`KismetMaterialLibrary.CreateDynamicMaterialInstance` (`PrimitiveComponent.GetMaterial` (`self.Bboxes`) 0)))
  (`MaterialInstanceDynamic.SetVectorParameterValue` _returnvalue "Color" (`self.Color`))
  (`PrimitiveComponent.SetMaterial` (`self.Bboxes`) 0 _returnvalue)
  ;[1 1 1] Set color of the plane and the text
  (bind _returnvalue_2 (`KismetMaterialLibrary.CreateDynamicMaterialInstance` (`PrimitiveComponent.GetMaterial` (`self.BackgroundBorder`) 0) "Color"))
  (`MaterialInstanceDynamic.SetVectorParameterValue` _returnvalue_2 "Color" (`self.Color`))
  (`PrimitiveComponent.SetMaterial` (`self.BackgroundBorder`) 0 _returnvalue_2)
  (`TextRenderComponent.SetTextRenderColor` (`self.TextRender`) (`KismetMathLibrary.Conv_LinearColorToColor` (`self.Color`))))

(fn `UserConstructionScript`)