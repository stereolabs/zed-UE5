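; Visualizes ZED body tracking by driving one spawned avatar per detected person.
; On each new detection frame it spawns or updates avatars by object ID, feeding data to ABP_Avatar_FootIK, and destroys those no longer detected.
; Optional height matching stretches avatar Z once, from tracked neck height over bone height, passing the inverse scale to the AnimBP.
; It also adds the camera image canvas and can auto-start object detection.
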(event `Disable OD`
  ;[1 1 1] Create Enable/Disable OD button in Editor
  (`ZEDCamera.DisableObjectDetection` (`ZEDFunctionLibrary.GetCameraActor`)))

(event `Enable OD`
  ;[1 1 1] Create Enable/Disable OD button in Editor
  (`ZEDCamera.EnableObjectDetection` (`ZEDFunctionLibrary.GetCameraActor`)))

(event `OnTrackingEnabled_Event_0`
  (params (bSuccess :type Boolean) (ErrorCode :type "ESlErrorCode Enum" :default "EC_Success") (Location :type "Vector Structure (by ref)") (Rotation :type "Rotator Structure (by ref)"))
  ;[1 1 1] Enable OD automaticcly when the camera is ready (when tracking is enabled)
  (if (`self.StartObjectDetectionAutomatically`)
    (`ZEDCamera.EnableObjectDetection` (`ZEDFunctionLibrary.GetCameraActor`))))

(event `self.ReceiveBeginPlay`
  (`|ExecutionSequence`
    (:`then_0`
      ;[1 1 1] Enable OD automaticcly when the camera is ready (when tracking is enabled)
      (add `SlCameraProxy.OnTrackingEnabled` (`SlFunctionLibrary.GetCameraProxy`) (delegate `OnTrackingEnabled_Event_0`)))
    (:`then_1`
      ;[1 1 1] Create canvas to display ZED Image on the screen
      (bind _returnvalue (`|CreateWidget` "/Game/ZED/Blueprints/BodyTracking/BP_VirtualCanvas.BP_VirtualCanvas_C"))
      (`UserWidget.AddToViewport` _returnvalue 0))
    (:`then_2`
      ;[1 1 1] Bind event to retrieve object function
      (add `SlCameraProxy.OnObjectDetectionRetrieved` (`SlFunctionLibrary.GetCameraProxy`) (delegate `OnObjectDetectionRetrieved_Event_1`)))))

(event `OnObjectDetectionRetrieved_Event_1`
  (params (objects :type "SlObjects Structure (by ref)"))
  (bind (_timestamp _objectslist _bisnew) (break `SlObjects` objects))
  (bind _spheres (`self.Spheres`))
  (bind _value (`BlueprintMapLibrary.Map_Find` (`self.Avatars`) (`self.Id`)))
  (bind _returnvalue (/ (`.Z` (`KismetMathLibrary.BreakVector3f` (`|GetArrayItem` (`.Keypoint` (break `SlObjectData` (`self.Current Object`))) (`KismetMathLibrary.Conv_ByteToInt` (`ZEDFunctionLibrary.GetIndexFromValuePose34` "NECK"))))) (`BlueprintMapLibrary.Map_Find` (`self.AvatarHeight`) (`self.Id`))))
  (bind _returnvalue_2 (`KismetMathLibrary.MakeVector` 1.0 1.0 _returnvalue))
  ;[1 1 1] Bind event to retrieve object function
  (if _bisnew
    ;[1 1 1] Fill up the RemaningAvatars array.
    ; Used to know which person is no longer detected in the scene and destroy its avatar
    (bind _keys (`BlueprintMapLibrary.Map_Keys` (`self.Avatars`)))
    (set `self.Remaining Avatars` _keys)
    (for _array_element _objectslist
      (set `self.Current Object` _array_element)
      (bind (_id _uniqueobjectid _rawlabel _label _sublabel _trackingstate) (break `SlObjectData` _array_element))
      (set `self.Id` _id)
      ;[1 1 1] If Tracking State is OK
      (if (`|EnumEquality` _trackingstate "OTS_Ok")
        (if (`BlueprintMapLibrary.Map_Contains` (`self.Avatars`) _id)
          (`KismetArrayLibrary.Array_RemoveItem` (`self.Remaining Avatars`) (`self.Id`))
          ;[1 1 1] If the Avatar is already in the scene, only update its Skeletal Mesh
          (bind _output_get (set `self.Skeletal Mesh` (`self.GetComponentByClass` _value "/Script/Engine.SkeletalMeshComponent")))
          (bind _asbp_avatar_full_body_ik_anim_blueprint (cast `/Game/ZED/Blueprints/BodyTracking/ABP_Avatar_FootIK` (`SkeletalMeshComponent.GetAnimInstance` _output_get))
            (:`then`
              (set `/Game/ZED/Blueprints/BodyTracking/ABP_Avatar_FootIK.Object Data` (`self.Current Object`) _asbp_avatar_full_body_ik_anim_blueprint)
              (if (`self.MatchBodyHeight`)
                (if (> (`BlueprintMapLibrary.Map_Find` (`self.Scale`) (`self.Id`)) 0.0)
                  _
                  (elif (not (== _returnvalue 0.0))
                    (`BlueprintMapLibrary.Map_Add` (`self.Scale`) (`self.Id`) _returnvalue)
                    (`self.SetActorScale3D` _value _returnvalue_2)
                    (set `/Game/ZED/Blueprints/BodyTracking/ABP_Avatar_FootIK.Scale` (/ (1.0 1.0 1.0) _returnvalue_2) _asbp_avatar_full_body_ik_anim_blueprint)))))
            (:`CastFailed`
              (`KismetSystemLibrary.PrintString` "CAST FAILED! BPAVATARFBIKANIMBP Update")))
          (else
            ;[1 1 1] New Detection : Spawn a new Avatar and update its Skeletal Mesh with Body Tracking Data
            (bind _returnvalue_3 (`|SpawnActorFromClass` (`self.Avatar`) (`self.Spawn Transform`) "Undefined" "OverrideRootScale" null null))
            (`BlueprintMapLibrary.Map_Add` (`self.Avatars`) (`self.Id`) _returnvalue_3)
            (bind _output (`|GetArrayItem` (`self.GetComponentsByTag` _returnvalue_3 "/Script/Engine.SkeletalMeshComponent" "OriginalSM")))
            (bind _asbp_avatar_full_body_ik_anim_blueprint_2 (cast `/Game/ZED/Blueprints/BodyTracking/ABP_Avatar_FootIK` (`SkeletalMeshComponent.GetAnimInstance` _output))
              (:`then`
                (set `/Game/ZED/Blueprints/BodyTracking/ABP_Avatar_FootIK.Object Data` (`self.Current Object`) _asbp_avatar_full_body_ik_anim_blueprint_2)
                (`BlueprintMapLibrary.Map_Add` (`self.Scale`) (`self.Id`))
                (bind _returnvalue_4 (`SlFunctionLibrary.GetSkeletonBoneHeight` _output "Neck"))
                (`BlueprintMapLibrary.Map_Add` (`self.AvatarHeight`) (`self.Id`) _returnvalue_4))
              (:`CastFailed`
                (`KismetSystemLibrary.PrintString` "CAST FAILED! BPAVATARFBIKANIMBP CREAT")))))))
    ;[1 1 1] Destroy Avatars which are not longer detected in the scene
    (for _array_element_2 (`self.Remaining Avatars`)
      (bind (_value_2 _returnvalue_5) (`BlueprintMapLibrary.Map_Find` (`self.Avatars`) _array_element_2))
      (if (== _returnvalue_5 true)
        (`self.K2_DestroyActor` _value_2)
        (`BlueprintMapLibrary.Map_Remove` (`self.Avatars`) _array_element_2)
        (`BlueprintMapLibrary.Map_Remove` (`self.Scale`) (`self.Id`))
        (`self.K2_DestroyActor` _spheres)
        (`KismetArrayLibrary.Array_Clear` _spheres)))))

(fn `UserConstructionScript`)