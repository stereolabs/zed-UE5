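; Visualizes ZED body tracking by spawning one foot-IK avatar per tracked person.
; Adds the ZED image canvas to the viewport, optionally starts object detection when tracking is enabled, and has manual enable/disable events.
; Each new detection frame spawns or updates avatars keyed by ID, passing body data and smoothing settings to their ABP_ZED_Manny_FootIK anim instance.
; Avatars not in an OK tracking state that frame are destroyed.
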(event `Disable OD`
  ;[1 1 1] Create Enable/Disable OD button in Editor
  (`ZEDCamera.DisableObjectDetection` (`ZEDFunctionLibrary.GetCameraActor`)))

(event `Enable OD`
  ;[1 1 1] Create Enable/Disable OD button in Editor
  (`ZEDCamera.EnableObjectDetection` (`ZEDFunctionLibrary.GetCameraActor`)))

(event `OnTrackingEnabled_Event_0`
  (params (bSuccess :type Boolean) (ErrorCode :type "ESlErrorCode Enum" :default "EC_Success") (Location :type "Vector Structure (by ref)") (Rotation :type "Rotator Structure (by ref)"))
  ;[1 1 1] Enable OD automaticcly when the camera is ready (when tracking is enabled)
  (if (`self.StartObjectDetectionAutomatically`)
    (`ZEDCamera.EnableObjectDetection` (`ZEDFunctionLibrary.GetCameraActor`))))

(event `self.ReceiveBeginPlay`
  (`|ExecutionSequence`
    (:`then_0`
      ;[1 1 1] Enable OD automaticcly when the camera is ready (when tracking is enabled)
      (add `SlCameraProxy.OnTrackingEnabled` (`SlFunctionLibrary.GetCameraProxy`) (delegate `OnTrackingEnabled_Event_0`)))
    (:`then_1`
      ;[1 1 1] Create canvas to display ZED Image on the screen
      (bind _returnvalue (`|CreateWidget` "/Game/ZED/Blueprints/BodyTracking/BP_VirtualCanvas.BP_VirtualCanvas_C"))
      (`UserWidget.AddToViewport` _returnvalue 0))
    (:`then_2`
      ;[1 1 1] Bind event to retrieve object function
      (add `SlCameraProxy.OnObjectDetectionRetrieved` (`SlFunctionLibrary.GetCameraProxy`) (delegate `OnObjectDetectionRetrieved_Event_1`)))))

(event `OnObjectDetectionRetrieved_Event_1`
  (params (objects :type "SlObjects Structure (by ref)"))
  (bind (_timestamp _objectslist _bisnew) (break `SlObjects` objects))
  ;[1 1 1] Bind event to retrieve object function
  (if _bisnew
    ;[1 1 1] Fill up the RemaningAvatars array.
    ; Used to know which person is no longer detected in the scene and destroy its avatar
    (bind _keys (`BlueprintMapLibrary.Map_Keys` (`self.Avatars`)))
    (set `self.Remaining Avatars` _keys)
    (for _array_element _objectslist
      (set `self.Current Object` _array_element)
      (bind (_id _uniqueobjectid _rawlabel _label _sublabel _trackingstate) (break `SlObjectData` _array_element))
      (set `self.Id` _id)
      ;[1 1 1] If Tracking State is OK
      (if (`|EnumEquality` _trackingstate "OTS_Ok")
        (if (`BlueprintMapLibrary.Map_Contains` (`self.Avatars`) _id)
          (`KismetArrayLibrary.Array_RemoveItem` (`self.Remaining Avatars`) (`self.Id`))
          ;[1 1 1] If the Avatar is already in the scene, only update its Skeletal Mesh
          (bind _output_get (set `self.Skeletal Mesh` (`self.GetComponentByClass` (`BlueprintMapLibrary.Map_Find` (`self.Avatars`) (`self.Id`)) "/Script/Engine.SkeletalMeshComponent")))
          (bind _asabp_zed_manny_foot_ik (cast `/Game/ZED/Blueprints/BodyTracking/ABP_ZED_Manny_FootIK` (`SkeletalMeshComponent.GetAnimInstance` _output_get) :!pure true))
          (set `/Game/ZED/Blueprints/BodyTracking/ABP_ZED_Manny_FootIK.Object Data` (`self.Current Object`) _asabp_zed_manny_foot_ik)
          (set `/Game/ZED/Blueprints/BodyTracking/ABP_ZED_Manny_FootIK.Skeletal Mesh` (`self.Skeletal Mesh`) _asabp_zed_manny_foot_ik)
          (`self.UpdateSmoothingParams` _asabp_zed_manny_foot_ik)
          (else
            ;[1 1 1] New Detection : Spawn a new Avatar and update its Skeletal Mesh with Body Tracking Data
            (bind _returnvalue (`|SpawnActorFromClass` (`self.Actor Class`) (`self.Spawn Transform`) "Undefined" "OverrideRootScale" null null))
            (`BlueprintMapLibrary.Map_Add` (`self.Avatars`) (`self.Id`) _returnvalue)
            (bind _returnvalue_2 (`self.GetComponentByClass` _returnvalue "/Script/Engine.SkeletalMeshComponent"))
            (set `self.Skeletal Mesh` _returnvalue_2)
            (bind _asbp_avatar_foot_ik (cast `/Game/ZED/Blueprints/BodyTracking/BP_Avatar_FootIK` _returnvalue))
            (`/Game/ZED/Blueprints/BodyTracking/BP_Avatar_FootIK.ToggleSelfCollision` _asbp_avatar_foot_ik (`self.EnableSelfCollision`))
            (bind _asabp_zed_manny_foot_ik_2 (cast `/Game/ZED/Blueprints/BodyTracking/ABP_ZED_Manny_FootIK` (`SkeletalMeshComponent.GetAnimInstance` _returnvalue_2) :!pure true))
            (set `/Game/ZED/Blueprints/BodyTracking/ABP_ZED_Manny_FootIK.Object Data` (`self.Current Object`) _asabp_zed_manny_foot_ik_2)
            (set `/Game/ZED/Blueprints/BodyTracking/ABP_ZED_Manny_FootIK.Skeletal Mesh` (`self.Skeletal Mesh`) _asabp_zed_manny_foot_ik_2)
            (`self.UpdateSmoothingParams` _asabp_zed_manny_foot_ik_2)))))
    ;[1 1 1] Destroy Avatars which are not longer detected in the scene
    (for _array_element_2 (`self.Remaining Avatars`)
      (bind (_value _returnvalue_3) (`BlueprintMapLibrary.Map_Find` (`self.Avatars`) _array_element_2))
      (if (== _returnvalue_3 true)
        (`self.K2_DestroyActor` _value)
        (`BlueprintMapLibrary.Map_Remove` (`self.Avatars`) _array_element_2)))))

(fn `UpdateSmoothingParams`
  (params (ABP_ZED_Manny_FootIK :type "/Game/ZED/Blueprints/BodyTracking/ABP_ZED_Manny_FootIK Object Reference"))
  (set `/Game/ZED/Blueprints/BodyTracking/ABP_ZED_Manny_FootIK.Rotation Slerp Intensity` (`self.JointRotationSmoothing`) ABP_ZED_Manny_FootIK)
  (set `/Game/ZED/Blueprints/BodyTracking/ABP_ZED_Manny_FootIK.Root Location Slerp Intensity` (`self.RootTranslationSmoothing`) ABP_ZED_Manny_FootIK))

(fn `UserConstructionScript`)