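; ZED body-tracking skeleton actor that draws a tracked person as 18 colored spheres and hides its skeletal mesh.
; BeginPlay spawns and attaches the spheres in random colors, optionally one shared color, and functions move or toggle them.
; Keypoint updates accept 18- or 34-point poses, remapping 34 down to 18 for nodes.
; Cylinder bone functions exist, but bone spawning is disconnected and the 18-point path always moves bone 0.
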(event `self.ReceiveBeginPlay`
  (bind _skeletalmesh (`self.SkeletalMesh`))
  (`|ExecutionSequence`
    (:`then_0`
      (`PrimitiveComponent.SetCollisionEnabled` _skeletalmesh "NoCollision")
      (`SceneComponent.SetVisibility` _skeletalmesh false true))
    (:`then_1`
      ;[1 1 1] Fill array of node nodes actors (spheres)
      (for _index (range 18)
        (bind _returnvalue (`|SpawnActorFromClass` "/Game/ZED/Blueprints/BodyTracking/BP_CustomSphere.BP_CustomSphere_C" (`KismetMathLibrary.MakeTransform` (`SceneComponent.K2_GetComponentLocation` (`self.Root`)) (struct) (0.6 0.6 0.6)) "AlwaysSpawn" "OverrideRootScale" null null))
        (`MeshComponent.SetVectorParameterValueOnMaterials` (`StaticMeshActor.StaticMeshComponent` _returnvalue) "MaterialColor" (`self.GiveColorDependingOnIndex` _index))
        (`self.K2_AttachToActor` _returnvalue self "None" "KeepRelative" "KeepRelative" "KeepRelative" true)
        (`KismetArrayLibrary.Array_Add` (`self.Nodes`) _returnvalue)))))

(fn `GiveColorDependingOnIndex`
  (params (Index :type Integer))
  (returns (Color :type "Vector Structure"))
  (bind _returnvalue (`KismetMathLibrary.MakeVector` (`KismetMathLibrary.RandomFloat`) (`KismetMathLibrary.RandomFloat`) (`KismetMathLibrary.RandomFloat`)))
  (if (`self.SameColorForEverything`)
    (if (`self.ColorInitialized`)
      (return (`self.SameColor`))
      (else
        (bind _output_get (set `self.SameColor` _returnvalue))
        (set `self.ColorInitialized` true)
        (return _output_get)))
    (else
      (return _returnvalue))))

(fn `MoveBonesToKeypoints`
  (params (KeypointsLocations :type "Array of Vector Structure"))
  (bind _output_get (set `self.KeypointsLocs` KeypointsLocations))
  ;[1 1 1] Check Pose34
  (if (== (`KismetArrayLibrary.Array_Length` _output_get) 34)
    (for (_array_element _array_index) (`ZEDFunctionLibrary.GetBodyBonesPose34`)
      (bind (_firstend _secondend) (break `SlBone34` _array_element))
      (`self.MoveBoneTo` (`|GetArrayItem` (`self.KeypointsLocs`) (`KismetMathLibrary.Conv_ByteToInt` _firstend)) (`|GetArrayItem` (`self.KeypointsLocs`) (`KismetMathLibrary.Conv_ByteToInt` _secondend)) _array_index))
    (else
      (for _array_element_2 (`ZEDFunctionLibrary.GetBodyBonesPose18`)
        (bind (_firstend_2 _secondend_2) (break `SlBone18` _array_element_2))
        (`self.MoveBoneTo` (`|GetArrayItem` (`self.KeypointsLocs`) (`KismetMathLibrary.Conv_ByteToInt` _firstend_2)) (`|GetArrayItem` (`self.KeypointsLocs`) (`KismetMathLibrary.Conv_ByteToInt` _secondend_2)))))))

(fn `MoveBoneTo`
  (params (NewLoc1 :type "Vector Structure") (NewLoc2 :type "Vector Structure") (Index :type Integer))
  (`/Game/ZED/Blueprints/BodyTracking/BP_CustomCylinder.MoveTo` (`|GetArrayItem` (`self.Bones`) Index) NewLoc1 NewLoc2))

(fn `MoveNodesToKeypoints`
  (params (KeypointsLocations :type "Array of Vector Structure"))
  (locals (KPs18in34 :type "Array of Integer") (Counter34 :type Integer))
  (set `self.KeypointsLocs` KeypointsLocations)
  (if (== (`KismetArrayLibrary.Array_Length` KeypointsLocations) 34)
    (for (_ _array_index) (`self.Nodes`)
      (`self.MoveNodeTo` _array_index (`|GetArrayItem` (`self.KeypointsLocs`) (`|GetArrayItem` (`local.KPs18in34`) _array_index))))
    (else
      ;[1 1 1] 18 keypoints
      (for (_ _array_index_2) (`self.Nodes`)
        (`self.MoveNodeTo` _array_index_2 (`|GetArrayItem` (`self.KeypointsLocs`) _array_index_2))))))

(fn `MoveNodeTo`
  (params (IndexNode :type Integer) (NewLocation :type "Vector Structure"))
  (`SceneComponent.K2_SetWorldLocation` (`Actor.RootComponent` (`|GetArrayItem` (`self.Nodes`) IndexNode)) NewLocation false false))

(fn `ShowBones`
  (params (ShouldShow :type Boolean) (ShouldCollide :type "ECollisionEnabled Enum" :default "NoCollision"))
  (if ShouldShow
    (for _array_element (`self.Bones`)
      (bind _returnvalue (`self.GetComponentByClass` _array_element "/Script/Engine.StaticMeshComponent"))
      (`PrimitiveComponent.SetCollisionEnabled` _returnvalue ShouldCollide)
      (`SceneComponent.SetVisibility` _returnvalue ShouldShow false)
      (set `self.IsBonesVisible` ShouldShow :!label _label))
    (else
      (for _array_element_2 (`self.Bones`)
        (bind _returnvalue_2 (`self.GetComponentByClass` _array_element_2 "/Script/Engine.StaticMeshComponent"))
        (`PrimitiveComponent.SetCollisionEnabled` _returnvalue_2 ShouldCollide)
        (`SceneComponent.SetVisibility` _returnvalue_2 ShouldShow false)
        (goto _label)))))

(fn `ShowNodes`
  (params (ShouldShow :type Boolean) (ShouldCollide :type "ECollisionEnabled Enum" :default "NoCollision"))
  (if ShouldShow
    (for _array_element (`self.Nodes`)
      (bind _returnvalue (`self.GetComponentByClass` _array_element "/Script/Engine.StaticMeshComponent"))
      (`PrimitiveComponent.SetCollisionEnabled` _returnvalue ShouldCollide)
      (`SceneComponent.SetVisibility` _returnvalue ShouldShow false)
      (set `self.IsNodesVisible` ShouldShow))
    (else
      (for _array_element_2 (`self.Nodes`)
        (bind _returnvalue_2 (`self.GetComponentByClass` _array_element_2 "/Script/Engine.StaticMeshComponent"))
        (`PrimitiveComponent.SetCollisionEnabled` _returnvalue_2 ShouldCollide)
        (`SceneComponent.SetVisibility` _returnvalue_2 ShouldShow false)
        (set `self.IsNodesVisible` ShouldShow)))))

(fn `UserConstructionScript`)