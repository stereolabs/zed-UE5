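; Visualizes people detected by ZED camera object detection as skeleton actors in the scene, with optional auto-start once tracking is enabled.
; Each new detection result spawns or updates a BP_SDK_Skeleton per tracked ID, moving its joints and bones to the keypoints.
; An ID-keyed map is diffed each update to destroy skeletons, and their attached actors, no longer detected.
; Events enable or disable detection and toggle skeleton visibility and collision.
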(event `Disable OD`
  ;[1 1 1] Create Enable/Disable OD button in Editor
  (`ZEDCamera.DisableObjectDetection` (`ZEDFunctionLibrary.GetCameraActor`))
  (`self.DisableAvatarsOnODEnd`))

(event `Enable OD`
  ;[1 1 1] Create Enable/Disable OD button in Editor
  (`ZEDCamera.EnableObjectDetection` (`ZEDFunctionLibrary.GetCameraActor`)))

(event `OnTrackingEnabled_Event_0`
  (params (bSuccess :type Boolean) (ErrorCode :type "ESlErrorCode Enum" :default "EC_Success") (Location :type "Vector Structure (by ref)") (Rotation :type "Rotator Structure (by ref)"))
  ;[1 1 1] Enable OD automaticcly when the camera is ready (when tracking is enabled)
  (if (`self.StartObjectDetectionAutomatically`)
    (`ZEDCamera.EnableObjectDetection` (`ZEDFunctionLibrary.GetCameraActor`))))

(event `self.ReceiveBeginPlay`
  (`|ExecutionSequence`
    (:`then_0`
      ;[1 1 1] Enable OD automaticcly when the camera is ready (when tracking is enabled)
      (add `SlCameraProxy.OnTrackingEnabled` (`SlFunctionLibrary.GetCameraProxy`) (delegate `OnTrackingEnabled_Event_0`)))
    (:`then_1`
      (if false
        ;[1 1 1] Create canvas to display ZED Image on the screen
        (bind _returnvalue (`|CreateWidget` "/Game/ZED/Blueprints/BodyTracking/BP_VirtualCanvas.BP_VirtualCanvas_C"))
        (`UserWidget.AddToViewport` _returnvalue 0)))
    (:`then_2`
      ;[1 1 1] Bind event to retrieve object function
      (add `SlCameraProxy.OnObjectDetectionRetrieved` (`SlFunctionLibrary.GetCameraProxy`) (delegate `OnObjectDetectionRetrieved_Event_1`)))
    (:`then_3`
      (set `self.CollisionToSet` (`self.EnableCollision`)))))

(event `OnObjectDetectionRetrieved_Event_1`
  (params (objects :type "SlObjects Structure (by ref)"))
  (bind (_timestamp _objectslist _bisnew) (break `SlObjects` objects))
  ;[1 1 1] Bind event to retrieve object function
  (if _bisnew
    ;[1 1 1] Fill up the RemaningAvatars array.
    ; Used to know which person is no longer detected in the scene and destroy its avatar
    (bind _keys (`BlueprintMapLibrary.Map_Keys` (`self.Avatars`)))
    (set `self.Remaining Avatars` _keys)
    (for _array_element _objectslist
      (set `self.Current Object` _array_element)
      (bind (_id _uniqueobjectid _rawlabel _label _sublabel _trackingstate _actionstate _position _velocity _positioncovariance _boundingbox2d _mask _confidence _boundingbox _dimensions _keypoint2d _keypoint) (break `SlObjectData` _array_element))
      (set `self.Id` _id)
      (set `self.CurrentKeypoints` _keypoint)
      ;[1 1 1] If Tracking State is OK
      (if (`|EnumEquality` _trackingstate "OTS_Ok")
        (if (`BlueprintMapLibrary.Map_Contains` (`self.Avatars`) _id)
          (`KismetArrayLibrary.Array_RemoveItem` (`self.Remaining Avatars`) (`self.Id`))
          ;[1 1 1] If the avatar is already in the scene, only update its skeleton nodes
          (bind _asbp_sdk_skeleton (cast `/Game/ZED/Blueprints/BodyTracking/BP_SDK_Skeleton` (`BlueprintMapLibrary.Map_Find` (`self.Avatars`) (`self.Id`))))
          (`/Game/ZED/Blueprints/BodyTracking/BP_SDK_Skeleton.MoveNodesToKeypoints` _asbp_sdk_skeleton (`self.CurrentKeypoints`))
          (`/Game/ZED/Blueprints/BodyTracking/BP_SDK_Skeleton.MoveBonesToKeypoints` _asbp_sdk_skeleton (`self.CurrentKeypoints`))
          (else
            ;[1 1 1] Create the avatar if it does not exist yet
            (bind _returnvalue (`|SpawnActorFromClass` "/Game/ZED/Blueprints/BodyTracking/BP_SDK_Skeleton.BP_SDK_Skeleton_C" (`self.Spawn Transform`) "Undefined" "OverrideRootScale" null (`self.OneColorPerSkeleton`) null))
            (`BlueprintMapLibrary.Map_Add` (`self.Avatars`) (`self.Id`) _returnvalue)
            (`/Game/ZED/Blueprints/BodyTracking/BP_SDK_Skeleton.ShowNodes` _returnvalue (and (`self.ShowSkeletonJoints`) (`self.AvatarsVisible`)) (`self.CollisionToSet`))
            (`/Game/ZED/Blueprints/BodyTracking/BP_SDK_Skeleton.MoveNodesToKeypoints` _returnvalue (`self.CurrentKeypoints`))
            (`/Game/ZED/Blueprints/BodyTracking/BP_SDK_Skeleton.ShowBones` _returnvalue (and (`self.ShowSkeletonBones`) (`self.AvatarsVisible`)) (`self.CollisionToSet`))
            (`/Game/ZED/Blueprints/BodyTracking/BP_SDK_Skeleton.MoveBonesToKeypoints` _returnvalue (`self.CurrentKeypoints`))))))
    (`self.DestroyAllAvatars`)))

(event `DestroyAllAvatars`
  ;[1 1 1] Destroy avatars no longer detected in the scene
  (for _array_element (`self.Remaining Avatars`)
    (bind (_value _returnvalue) (`BlueprintMapLibrary.Map_Find` (`self.Avatars`) _array_element))
    (if _returnvalue
      (bind _outactors (`self.GetAttachedActors` _value false false))
      (while (> (`KismetArrayLibrary.Array_Length` _outactors) 0)
        (`self.K2_DestroyActor` (`|GetArrayItem` _outactors)))
      (`self.K2_DestroyActor` _value)
      (`BlueprintMapLibrary.Map_Remove` (`self.Avatars`) _array_element) ; remove no longer detected ids
    )))

(event `DisableAvatarsOnODEnd`
  ;[1 1 1] Destroy avatars no longer detected in the scene
  (bind _keys (`BlueprintMapLibrary.Map_Keys` (`self.Avatars`)))
  (for _array_element _keys
    (bind (_value _returnvalue) (`BlueprintMapLibrary.Map_Find` (`self.Avatars`) _array_element))
    (if _returnvalue
      (bind _outactors (`self.GetAttachedActors` _value false false))
      (while (> (`KismetArrayLibrary.Array_Length` _outactors) 0)
        (`self.K2_DestroyActor` (`|GetArrayItem` _outactors)))
      (`self.K2_DestroyActor` _value)
      (`BlueprintMapLibrary.Map_Remove` (`self.Avatars`) _array_element) ; remove no longer detected ids
    )))

(event `ToggleSkeletonVisibility`
  (params (Visibility :type Boolean))
  (bind _output_get (set `self.AvatarsVisible` Visibility))
  (if _output_get
    (set `self.CollisionToSet` (`self.EnableCollision`))
    (else
      (set `self.CollisionToSet` "NoCollision")))
  (`KismetSystemLibrary.PrintString` (`KismetStringLibrary.Concat_StrStr` "Skeleton ToggleVisibility [" (`KismetStringLibrary.Conv_BoolToString` Visibility) "]"))
  (bind _values (`BlueprintMapLibrary.Map_Values` (`self.Avatars`)))
  (for _array_element _values
    (bind _asbp_sdk_skeleton (cast `/Game/ZED/Blueprints/BodyTracking/BP_SDK_Skeleton` _array_element))
    (`/Game/ZED/Blueprints/BodyTracking/BP_SDK_Skeleton.ShowNodes` _asbp_sdk_skeleton Visibility (`self.CollisionToSet`))
    (`/Game/ZED/Blueprints/BodyTracking/BP_SDK_Skeleton.ShowBones` _asbp_sdk_skeleton Visibility (`self.CollisionToSet`))))

(fn `UpdateNodesAndBonesVisibilityAndCollision`
  (bind _collisiontoset (`self.CollisionToSet`))
  (bind _values (`BlueprintMapLibrary.Map_Values` (`self.Avatars`)))
  (for _array_element _values
    (bind _asbp_sdk_skeleton (cast `/Game/ZED/Blueprints/BodyTracking/BP_SDK_Skeleton` _array_element))
    (`/Game/ZED/Blueprints/BodyTracking/BP_SDK_Skeleton.ShowNodes` _asbp_sdk_skeleton (and (`self.ShowSkeletonJoints`) (`self.AvatarsVisible`)) _collisiontoset)
    (`/Game/ZED/Blueprints/BodyTracking/BP_SDK_Skeleton.ShowBones` _asbp_sdk_skeleton (and (`self.ShowSkeletonBones`) (`self.AvatarsVisible`)) _collisiontoset)))

(fn `UserConstructionScript`)