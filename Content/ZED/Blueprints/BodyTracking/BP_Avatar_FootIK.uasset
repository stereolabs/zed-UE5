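; BP_Avatar_FootIK is a ZED body-tracking avatar Blueprint whose graph adds optional self-clipping avoidance through physics-driven animation.
; On BeginPlay, if AvoidSelfClipping is set, it creates a Physical Animation Component and enables full-weight simulation on all bodies below Hips, excluding Hips.
; World-space physical animation drives then pull those bodies toward the animated pose.
; No foot IK logic appears in these graphs.
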(event `self.ReceiveBeginPlay`
  (bind _skeletalmesh (`self.SkeletalMesh`))
  (bind _hips (`self.Hips`))
  (if (`self.AvoidSelfClipping`)
    (bind _returnvalue (`AddComponent|NODE_AddPhysicalAnimationComponent-0`))
    (set `self.Physical Animation Component` _returnvalue)
    (`PhysicalAnimationComponent.SetSkeletalMeshComponent` (`self.Physical Animation Component`) null)
    (`SkeletalMeshComponent.SetAllBodiesBelowSimulatePhysics` _skeletalmesh _hips true false)
    (`SkeletalMeshComponent.SetAllBodiesBelowPhysicsBlendWeight` _skeletalmesh _hips 1.0 false false)
    (`PhysicalAnimationComponent.ApplyPhysicalAnimationSettingsBelow` (`self.Physical Animation Component`) (`self.Hips`) (make `PhysicalAnimationData` false 3000.0 100.0 100.0 100.0) false)))

(fn `UserConstructionScript`)