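; Crosshair actor for the ZED camera that floats in front of the player at the depth of whatever is at image center.
; BeginPlay enables hit testing with depth and normals on the camera proxy, and EndPlay disables it.
; Tick samples depth at a fixed center pixel, offsets and clamps it, then positions the root, compensating off-center projection.
; A hardcoded-off branch uses viewport center and also aligns rotation to the surface normal.
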(event `self.ReceiveBeginPlay`
  ;[1 1 1] Enable hit test. Can be done in level blueprint
  (`SlCameraProxy.EnableHitTest` (`SlFunctionLibrary.GetCameraProxy`) true)
  (`SlCameraProxy.SetHitTestDepthAndNormals` (`SlFunctionLibrary.GetCameraProxy`) true true)
  (`self.EnableInput` (`GameplayStatics.GetPlayerController` 0)))

(event `self.ReceiveEndPlay`
  (params (EndPlayReason :type "EEndPlayReason Enum" :default "Destroyed"))
  ;[1 1 1] Always disable hit test before application quit
  (`SlCameraProxy.EnableHitTest` (`SlFunctionLibrary.GetCameraProxy`) false))

(event `self.ReceiveTick`
  (params (DeltaSeconds :type "Float (single-precision)"))
  (if true
    (`SceneComponent.K2_SetWorldLocation` (`self.DefaultSceneRoot`) (`ZEDFunctionLibrary.GetCenteredLocationInFrontOfPlayer` (`KismetMathLibrary.FMin` (- (`.Distance` (`ZEDFunctionLibrary.GetDepthAtScreenPosition` (`ZEDFunctionLibrary.GetPlayerController`) (640.0 360.0))) 5.0) 200.0)) false false)
    (else
      (`SceneComponent.K2_SetWorldLocation` (`self.DefaultSceneRoot`) (`ZEDFunctionLibrary.GetCenteredLocationInFrontOfPlayer` (`KismetMathLibrary.FMin` (- (`ZEDFunctionLibrary.GetDepthAtScreenPosition` (`ZEDFunctionLibrary.GetPlayerController`) (/ (`WidgetLayoutLibrary.GetViewportSize`) 2.0)) 15.0) 2000.0)) false false)
      (`SceneComponent.K2_SetWorldRotation` (`self.DefaultSceneRoot`) (`KismetMathLibrary.Conv_VectorToRotator` (+ (`ZEDFunctionLibrary.GetNormalAtScreenPosition` (`ZEDFunctionLibrary.GetPlayerController`) (/ (`WidgetLayoutLibrary.GetViewportSize`) 2.0)) (`self.RotationOffset`))) false false))))

(fn `UserConstructionScript`)